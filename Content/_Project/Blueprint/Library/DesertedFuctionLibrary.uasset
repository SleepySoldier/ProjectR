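; Blueprint function library of debug helpers for showing values and vectors at runtime.
; DebugPrintValue prints a "Name = Value" line in a chosen color, using the name as the print key so repeated calls replace the previous message.
; DebugDrawVector draws an arrow and text label for an offset vector from a start point, clamping its length and flattening it to Z zero for a top-down, planar view.
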(fn DebugPrintValue
  (params (ValueName :type Name) (Value :type String) (TextColor :type Linear%20Color%20Structure))
  (Development|PrintString (LocalVariables|Get__WorldContext) (Utilities|String|ToString(Text) (Utilities|Text|FormatText "{Name} =  {Value}" ValueName Value)) true true TextColor 2.0 ValueName))

(fn DebugDrawVector
  (params (LineStart :type Vector) (LineEnd :type Vector) (LineLength :type Float%20%28double-precision%29) (LineColor :type Linear%20Color%20Structure) (TextToShow :type String))
  (bind _returnvalue (Math|Vector|VectorClampSizeMax LineEnd LineLength))
  (bind _returnvalue_2 (* LineStart "1.000000,1.000000,0.000000"))
  (bind _returnvalue_3 (+ _returnvalue_2 _returnvalue))
  (bind _returnvalue_4 (* _returnvalue_3 "1.000000,1.000000,0.000000"))
  (Rendering|Debug|DrawDebugArrow (LocalVariables|Get__WorldContext) _returnvalue_2 _returnvalue_4 5.0 LineColor 0.0 5.0)
  (Rendering|Debug|DrawDebugString (LocalVariables|Get__WorldContext) _returnvalue_4 TextToShow 0 LineColor))