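; Magic projectile actor that flies at a configurable speed and gravity scale, applied to its ProjectileMovement in the construction script.
; On BeginPlay it sets its owner, ignores that owner when moving, and starts a fast looping timer.
; Each tick of the timer runs a zero-length sphere trace against selected object types at its current location.
; A hit fires the OnProjectileImpact dispatcher with the hit result, then destroys the projectile.
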(event Custom|ImpactTrace
  (bind _returnvalue (Transformation|GetActorLocation))
  (bind (_outhit _returnvalue_2) (Collision|SphereTraceForObjects _returnvalue _returnvalue (Variables|/Script/Engine.SphereComponent|GetSphereRadius (Variables|Default|GetSphere)) (Variables|Default|GetObjectTypesToAffect) false 0 "None"))
  (if _returnvalue_2
    (Default|CallOnProjectileImpact _outhit)
    (Actor|DestroyActor)))

(event EventBeginPlay
  (Actor|SetOwner (Variables|Default|GetNew%20Owner))
  (Utilities|Time|SetTimerbyEvent (delegate Custom|ImpactTrace) 0.01 true)
  (Collision|IgnoreActorwhenMoving (Variables|Default|GetSphere) (Components|GetOwner) true))

(fn ConstructionScript
  (bind _projectilemovement (Variables|Default|GetProjectileMovement))
  (bind _speed (Variables|Default|GetSpeed))
  (Variables|/Script/Engine.ProjectileMovementComponent|SetInitialSpeed _projectilemovement _speed)
  (Variables|/Script/Engine.ProjectileMovementComponent|SetMaxSpeed _projectilemovement _speed)
  (Variables|/Script/Engine.ProjectileMovementComponent|SetProjectileGravityScale _projectilemovement (Variables|Default|GetProjectile%20Gravity%20Scale)))