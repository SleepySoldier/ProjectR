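; Ranged enemy Blueprint that equips a weapon on BeginPlay and shoots at its attack target.
; Attack plays a montage and immediately fires a projectile-damage bullet through BPCAttacks, starting well forward of the rifle's muzzle socket, then calls AttackEnd on completion or interruption.
; Equip and unequip montage notifies drive weapon spawning, socket attachment and the equipped flag, with callbacks on blend out.
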(event EventUnequipWeapon
  (Animation|Montage|PlayMontage (Variables|Character|GetMesh) (Variables|Default|GetUnequipMontage)
    (:OnBlendOut
      (Default|CallOnUnequipWeapon))
    (:OnNotifyBegin
      (Transformation|AttachComponentToComponent (Variables|Default|GetWeaponComp) 0 "" "SnapToTarget" "SnapToTarget" "SnapToTarget" true)
      (Variables|Default|SetWeaponEquipped false))))

(event EventEquipWeapon
  (Animation|Montage|PlayMontage (Variables|Character|GetMesh) (Variables|Default|GetEquipMontage)
    (:OnBlendOut
      (Default|CallOnEquipWeapon))
    (:OnNotifyBegin
      (bind _returnvalue (Game|SpawnActorfromClass (Variables|Default|GetWeaponClass) (Math|Transform|MakeTransform "0, 0, 0" "0, 0, 0" "1.000000,1.000000,1.000000") "Undefined" "MultiplyWithRoot" self 0))
      (bind _output_get (Variables|Default|SetWeaponComp _returnvalue))
      (Transformation|AttachComponentToComponent _output_get (Variables|Character|GetMesh) (Variables|Default|GetWeaponSocketName) "SnapToTarget" "SnapToTarget" "SnapToTarget" true)
      (Variables|Default|SetWeaponEquipped true))))

(event EventBeginPlay
  (|CallParentFunction)
  (CallFunction|EquipWeapon))

(event EventAttack
  (params (AttackTarget :type Actor%20Object%20Reference))
  (|CallParentFunction AttackTarget)
  (Animation|Montage|PlayMontage (Variables|Character|GetMesh) (Variables|Default|GetAttackMontage)
    (:then
      (Default|FireBullet (Variables|Default|GetBPC_Attacks) (+ (Transformation|GetSocketLocation (Variables|/Game/_Project/Blueprint/Weapons/_BP_WeaponBase._BP_WeaponBase_C|GetSKM_Weapon (.AsBP%20Weapon%20Rifle (Utilities|Casting|CastToBP_Weapon_Rifle (Variables|Default|GetWeaponComp)))) "MuzzleFlash") (* (Transformation|GetActorForwardVector) 2e+03)) (Transformation|GetActorLocation AttackTarget) (Utilities|Struct|MakeDamageInfo 15.0 "Projectile" "HitReact" "0.000000,0.000000,0.000000" "None" false true false true self)))
    (:OnCompleted
      (CallFunction|AttackEnd AttackTarget :!label _label))
    (:OnInterrupted
      (goto _label))))

(fn ConstructionScript
  (|CallParentFunction))