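; Melee enemy character that equips a weapon via montages, blocks and delegates several attacks to an attacks component.
; Montage notifies attach or detach the weapon, and attack events pass montage and damage info for short-range, spin, jump and ground-slam moves.
; Blockable hits only roll for a timed block and return false without applying damage; others reach the damage system.
; Death turns the sword mesh into a physics object before parent handling.
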(event OnBlocked(BPC_DamageSystem)
  (params (CanBeParried :type Boolean) (DamageCauser :type Actor%20Object%20Reference))
  ;[0 0 0 0.5] Blocking
  (Variables|Default|SetBlockingState "NewEnumerator2")
  (Niagara|SpawnSystematLocation "/Niagara/DefaultAssets/Templates/Systems/DirectionalBurstLightweight.DirectionalBurstLightweight" (Transformation|GetSocketLocation (Variables|Character|GetMesh) "hand_r"))
  (Animation|Montage|PlayMontage (Variables|Character|GetMesh) "/Game/ThirdPerson/Characters/Mannequins/Anims/Sword/AM_Sword_Block.AM_Sword_Block"
    (:then
      (Utilities|Time|ClearandInvalidateTimerbyHandle (Variables|Default|GetHoldBlockTimerHandle)))
    (:OnCompleted
      (CallFunction|EndBlock :!label _label))
    (:OnInterrupted
      (goto _label))))

(event Custom|StartBlock
  ;[0 0 0 0.5] Blocking
  (Utilities|Time|ClearandInvalidateTimerbyHandle (Variables|Default|GetHoldBlockTimerHandle))
  (CallFunction|SetMovementSpeed "NewEnumerator2")
  (Variables|/Script/Project_R_Revival.DamageSystemComponent|SetbIsBlocking (Variables|Default|GetBPC_DamageSystem) true)
  (Variables|Default|SetBlockingState "NewEnumerator1")
  (bind _returnvalue (Utilities|Time|SetTimerbyEvent (EventDispatchers|CreateEvent :!event Custom|EndBlock) 2.0))
  (Variables|Default|SetHoldBlockTimerHandle _returnvalue))

(event Custom|EndBlock
  ;[0 0 0 0.5] Blocking
  (Variables|/Script/Project_R_Revival.DamageSystemComponent|SetbIsBlocking (Variables|Default|GetBPC_DamageSystem) false)
  (Variables|Default|SetBlockingState "NewEnumerator0")
  (CallFunction|SetMovementSpeed "NewEnumerator1")
  (Default|CallOnEndBlock))

(event Custom|SpinAttack
  (params (AttackTarget :type Actor%20Object%20Reference))
  ;[0 0 0 0.5] Attacking
  (Default|SpinAttack (Variables|Default|GetBPC_Attacks) (Utilities|Struct|MakeF_AttackInfo AttackTarget (Variables|Default|GetSpinAttackMontage) (Utilities|Struct|MakeDamageInfo 1e+01 "Melee" "HitReact" "0.000000,0.000000,0.000000" "None" false true true true))))

(event Custom|ShortRangedAttack
  (params (AttackTarget :type Actor%20Object%20Reference))
  ;[0 0 0 0.5] Attacking
  (Default|PrimaryMeleeAttack (Variables|Default|GetBPC_Attacks) (Utilities|Struct|MakeF_AttackInfo AttackTarget (Variables|Default|GetAttackMontage) (Utilities|Struct|MakeDamageInfo 15.0 "Melee" "HitReact" "0.000000,0.000000,0.000000" "None" false true true true)) 2e+02 3e+01))

(event Custom|LongRangeAttack
  (params (AttackTarget :type Actor%20Object%20Reference))
  ;[0 0 0 0.5] Attacking
  (Default|LongRangeMeleeAttack (Variables|Default|GetBPC_Attacks) (Utilities|Struct|MakeF_AttackInfo AttackTarget (Variables|Default|GetJumpAttackMontage) (Utilities|Struct|MakeDamageInfo 15.0 "Melee" "HitReact" "0.000000,0.000000,0.000000" "None" false true false true))))

(event Custom|GroundSmashAttack
  (params (AttackTarget :type Actor%20Object%20Reference))
  ;[0 0 0 0.5] Attacking
  (Default|GroundSlamAttack (Variables|Default|GetBPC_Attacks) (Utilities|Struct|MakeF_AttackInfo AttackTarget "/Game/ThirdPerson/Characters/Mannequins/Anims/Sword/AM_GroundSmash.AM_GroundSmash" (Utilities|Struct|MakeDamageInfo 25.0 "Explosion" "Knockback" "0.000000,0.000000,0.000000" "None" false false false true)) 3e+02))

(event EventUnequipWeapon
  (Animation|Montage|PlayMontage (Variables|Character|GetMesh) (Variables|Default|GetUnequipMontage)
    (:OnBlendOut
      (Default|CallOnUnequipWeapon))
    (:OnNotifyBegin
      (Transformation|AttachComponentToComponent (Variables|Default|GetWeaponComp) 0 "" "SnapToTarget" "SnapToTarget" "SnapToTarget" true)
      (Variables|Default|SetWeaponEquipped false))))

(event EventEquipWeapon
  (Animation|Montage|PlayMontage (Variables|Character|GetMesh) (Variables|Default|GetEquipMontage)
    (:OnBlendOut
      (Default|CallOnEquipWeapon))
    (:OnNotifyBegin
      (bind _returnvalue (Game|SpawnActorfromClass (Variables|Default|GetWeaponClass) (Math|Transform|MakeTransform "0, 0, 0" "0, 0, 0" "1.000000,1.000000,1.000000") "Undefined" "MultiplyWithRoot" self 0))
      (bind _output_get (Variables|Default|SetWeaponComp _returnvalue))
      (Transformation|AttachComponentToComponent _output_get (Variables|Character|GetMesh) (Variables|Default|GetWeaponSocketName) "SnapToTarget" "SnapToTarget" "SnapToTarget" true)
      (Variables|Default|SetWeaponEquipped true))))

(event EventBeginPlay
  (|CallParentFunction))

(event EventAttack
  (params (AttackTarget :type Actor%20Object%20Reference))
  ;[0 0 0 0.5] Attacking
)

(fn ConstructionScript
  (|CallParentFunction))

(fn TryBlock
  (if (Math|Random|RandomBoolwithWeight (Variables|Default|GetBlockChance))
    (CallFunction|StartBlock)))

(fn HandleDeath
  (bind _asbp_weapon_sword (Utilities|Casting|CastToBP_Weapon_Sword (Variables|Default|GetWeaponComp)))
  (Collision|SetCollisionEnabled (Variables|/Game/_Project/Blueprint/Weapons/_BP_WeaponBase._BP_WeaponBase_C|GetSM_Weapon _asbp_weapon_sword) "PhysicsOnly")
  (Physics|SetSimulatePhysics (Variables|/Game/_Project/Blueprint/Weapons/_BP_WeaponBase._BP_WeaponBase_C|GetSM_Weapon _asbp_weapon_sword) true)
  (|CallParentFunction))

(fn TakeDamage
  (params (DamageInfo :type Damage%20Info%20Structure%20%28by%20ref%29))
  (if (Utilities|Struct|BreakDamageInfo DamageInfo)
    (CallFunction|TryBlock)
    (return false)
    (else
      (bind _returnvalue (Class|DamageSystemComponent|TakeDamage (Variables|Default|GetBPC_DamageSystem) DamageInfo))
      (return _returnvalue))))