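; Lightning strike area-of-effect actor that shows a warning decal on the ground before it strikes.
; On BeginPlay it spawns the decal at its own location, waits DelayBeforeStrike, calls Trigger, then destroys the decal.
; Trigger is not implemented in these graphs, and the parent BeginPlay is left unconnected, so this sequence replaces any inherited startup logic.
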(event EventBeginPlay
  (bind _returnvalue (Rendering|Decal|SpawnDecalatLocation (Variables|Default|GetDecal%20Material) "256.000000,256.000000,0.000000" (Transformation|GetActorLocation) "-90.000000,0.000000,0.000000" 0.0))
  (Utilities|FlowControl|Delay (Variables|Default|GetDelayBeforeStrike))
  (CallFunction|Trigger)
  (Utilities|IsValid _returnvalue
    (:Is%20Valid
      (Components|DestroyComponent _returnvalue))))

(event Collision|EventActorBeginOverlap
  (params (OtherActor :type Actor%20Object%20Reference))
  (|CallParentFunction OtherActor) ; This node is disabled and will not be called.\nDrag off pins to build functionality.
)

(event EventTick
  (params (DeltaSeconds :type Float%20%28single-precision%29))
  (|CallParentFunction DeltaSeconds) ; This node is disabled and will not be called.\nDrag off pins to build functionality.
)

(fn ConstructionScript
  (|CallParentFunction))